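; BP_BloodStain is a blood stain clue object that reacts to stencil-highlight requests according to its RevealMode (None, Mania, Blindness or Both).
; TurnonStencil, when enabled, checks the incoming StencilID against that mode, with Mania matching 1 and Blindness 2.
; A match writes the stencil value to the mesh, but both outcomes turn custom depth off.
; A disabled request only prints debug text.
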(event EventBeginPlay)

(event Collision|EventActorBeginOverlap
  (params (OtherActor :type Actor%20Object%20Reference)))

(event EventTick
  (params (DeltaSeconds :type Float%20%28single-precision%29)))

(event EventTurnonStencil
  (params (Enabled :type Boolean) (StencilID :type Integer))
  (bind _staticmesh (Variables|Default|GetStaticMesh))
  (Development|PrintString "Enabled")
  (Development|PrintString (Utilities|String|ToString(Integer) StencilID))
  (if Enabled
    (switch Utilities|FlowControl|Switch|SwitchonE_RevealMode (Variables|Default|GetRevealMode)
      (:NewEnumerator0
        (Variables|Default|SetbAllow false))
      (:NewEnumerator1
        (Variables|Default|SetbAllow (== StencilID 1)))
      (:NewEnumerator2
        (Variables|Default|SetbAllow (== StencilID 2)))
      (:NewEnumerator3
        (Variables|Default|SetbAllow (or (== StencilID 1) (== StencilID 2)))))
    (if (Variables|Default|GetbAllow)
      (Rendering|SetRenderCustomDepth _staticmesh false)
      (Rendering|SetCustomDepthStencilValue _staticmesh StencilID)
      (else
        (Rendering|SetRenderCustomDepth _staticmesh false)))))

(fn ConstructionScript)