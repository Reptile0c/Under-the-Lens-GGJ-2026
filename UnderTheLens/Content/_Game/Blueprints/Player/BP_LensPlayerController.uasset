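; BP_LensPlayerController is a player controller that manages the mask wheel UI and reads movement input.
; BeginPlay adds the IMC_Lens input context, creates the WBP_Wheel widget and adds the first mask.
; Z, X, C keys and the EnabletheMasksUI event add further masks to the wheel.
; IA_Movement computes a clamped move scale and camera-relative planar direction, but applies no movement here.
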(event Input|EnhancedActionEvents|EnhancedInputActionIA_Movement
  (params (ActionValue :type Vector%202D%20Structure) (ElapsedSeconds :type Float%20%28double-precision%29) (TriggeredSeconds :type Float%20%28double-precision%29) (InputAction :type Input%20Action%20Object%20Reference :default "/Game/_Game/Input/IA_Movement.IA_Movement"))
  (bind _returnvalue (Game|GetPlayerCameraManager 0))
  (bind _returnvalue_2 (Math|Vector2D|Vector2DLength ActionValue))
  (bind (_x _y) (Math|Vector2D|BreakVector2D ActionValue))
  (bind _returnvalue_3 (Camera|GetCameraRotation _returnvalue))
  (bind _returnvalue_4 (Math|Vector|GetForwardVector _returnvalue_3))
  (bind _returnvalue_5 (Math|Vector|GetRightVector _returnvalue_3))
  (if (> _returnvalue_2 0.0)
    (Variables|Default|SetMoveScale (Math|Float|Clamp(Float) _returnvalue_2))
    (Variables|Default|SetMovementDirection (+ (* _x (Math|Vector|Normalize (Math|Vector|MakeVector (.x _returnvalue_4) (.y _returnvalue_4) 0.0))) (* _y (Math|Vector|Normalize (Math|Vector|MakeVector (.x _returnvalue_5) (.y _returnvalue_5) 0.0)))))))

(event EventBeginPlay
  (Input|AddMappingContext (PlayerController|LocalPlayerSubsystems|GetEnhancedInputLocalPlayerSubsystem) "/Game/_Game/Input/IMC_Lens.IMC_Lens" 0 "(bIgnoreAllPressedKeysUntilRelease=True,bForceImmediately=False,bNotifyUserSettings=False)")
  (bind _returnvalue (UserInterface|CreateWidget "/Game/_Game/Blueprints/Interaction/WBP_Wheel.WBP_Wheel_C"))
  (bind _output_get (Variables|Default|SetWheelRef _returnvalue))
  (UserInterface|Viewport|AddtoViewport _output_get 0)
  (Default|AddMask (Variables|Default|GetWheelRef) "NewEnumerator0"))

(event EventTick
  (params (DeltaSeconds :type Float%20%28single-precision%29)))

(event EventEnabletheMasksUI
  (params (Mask%20State :type E_MaskState%20Enum :default "NewEnumerator0"))
  (Default|AddMask (Variables|Default|GetWheelRef) Mask%20State))

(event Input|KeyboardEvents|X
  (params (Key :type Key%20Structure :default "None"))
  (:Pressed
    (Default|AddMask (Variables|Default|GetWheelRef) "NewEnumerator1")))

(event Input|KeyboardEvents|Z
  (params (Key :type Key%20Structure :default "None"))
  (:Pressed
    (Default|AddMask (Variables|Default|GetWheelRef) "NewEnumerator0")))

(event Input|KeyboardEvents|C
  (params (Key :type Key%20Structure :default "None"))
  (:Pressed
    (Default|AddMask (Variables|Default|GetWheelRef) "NewEnumerator2")))

(fn ConstructionScript)