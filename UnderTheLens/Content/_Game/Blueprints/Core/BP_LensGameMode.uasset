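; BP_LensGameMode is a game mode that tracks a game phase and handles the switch from main menu to gameplay.
; BeginPlay sets the initial phase and calls EnterMainMenu, which creates WI_Test with cursor and UI-only input, or only removes an existing menu.
; StartGame removes a valid menu, restores game-only input, hides the cursor and advances the phase.
; GameEnd is an empty stub.
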(event EventBeginPlay
  (Variables|Default|SetGamePhase "NewEnumerator0")
  (CallFunction|EnterMainMenu))

(event EventTick
  (params (DeltaSeconds :type Float%20%28single-precision%29)))

(fn ConstructionScript)

(fn StartGame
  (bind _returnvalue (Game|GetPlayerController 0))
  (bind _mainmenuwidgetref (Variables|Default|GetMainMenuWidgetRef))
  (Utilities|IsValid _mainmenuwidgetref
    (:Is%20Valid
      (Widget|RemovefromParent _mainmenuwidgetref)
      (Input|SetInputModeGameOnly _returnvalue false)
      (Variables|/Script/Engine.PlayerController|SetbShowMouseCursor _returnvalue false)
      (Variables|Default|SetGamePhase "NewEnumerator1"))))

(fn GameEnd)

(fn EnterMainMenu
  (bind _returnvalue (Game|GetPlayerController 0))
  (Utilities|IsValid (Variables|Default|GetMainMenuWidgetRef)
    (:Is%20Valid
      (Widget|RemovefromParent (Variables|Default|GetMainMenuWidgetRef)))
    (:Is%20Not%20Valid
      (bind _returnvalue_2 (UserInterface|CreateWidget "/Game/_Game/UI/WI_Test.WI_Test_C" _returnvalue))
      (bind _output_get (Variables|Default|SetMainMenuWidgetRef _returnvalue_2))
      (UserInterface|Viewport|AddtoViewport _output_get 0)
      (Variables|/Script/Engine.PlayerController|SetbShowMouseCursor _returnvalue true)
      (Input|SetInputModeUIOnly _returnvalue _output_get "DoNotLock" false))))