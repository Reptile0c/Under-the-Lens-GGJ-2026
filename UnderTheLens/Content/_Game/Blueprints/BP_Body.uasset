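; BP_Body is a body bag prop that appears only while the player's mask state is Blindness.
; It caches the player character on BeginPlay and polls the mask state every Tick to toggle mesh visibility.
; Collision starts disabled and turns on the first time anything leaves its trigger, or through the EnableCollison event, independent of visibility.
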(event OnComponentEndOverlap(CollisionTrigger)
  (params (OverlappedComponent :type Primitive%20Component%20Object%20Reference) (OtherActor :type Actor%20Object%20Reference) (OtherComp :type Primitive%20Component%20Object%20Reference) (OtherBodyIndex :type Integer))
  (if (not (Variables|Default|GetActivateCollision))
    (Collision|SetCollisionEnabled (Variables|Default|GetUTL_Props_BodyBag) "QueryAndPhysics")
    (Variables|Default|SetActivateCollision true)))

(event Custom|Enable%20Collison
  (Collision|SetCollisionEnabled (Variables|Default|GetUTL_Props_BodyBag) "QueryAndPhysics"))

(event EventTick
  (params (DeltaSeconds :type Float%20%28single-precision%29))
  (bind _utl_props_bodybag (Variables|Default|GetUTL_Props_BodyBag))
  (switch Utilities|FlowControl|Switch|SwitchonE_MaskState (Variables|/Game/_Game/Blueprints/BP_Player_NM.BP_Player_NM_C|GetCurrentMaskState (Variables|Default|GetAs%20BP%20Player%20NM))
    (:NewEnumerator0
      (Rendering|SetVisibility _utl_props_bodybag false false :!label _label))
    (:NewEnumerator1
      (goto _label))
    (:NewEnumerator2
      (Rendering|SetVisibility _utl_props_bodybag true false))
    (:NewEnumerator3
      (goto _label))))

(event EventBeginPlay
  (Rendering|SetVisibility (Variables|Default|GetUTL_Props_BodyBag) false false)
  (Collision|SetCollisionEnabled (Variables|Default|GetUTL_Props_BodyBag) "NoCollision")
  (bind _asbp_player_nm (Utilities|Casting|CastToBP_Player_NM (Game|GetPlayerCharacter 0)))
  (Variables|Default|SetAs%20BP%20Player%20NM _asbp_player_nm))

(fn ConstructionScript)