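; BP_RedWine is an interactable cleaning task whose appearance depends on the player's mask state.
; Every tick it shows a flowerpot in Normal or a carving knife in Mania, and updates the prompt widget text to match.
; A box overlap toggles the prompt's visibility.
; While overlapping in Mania, holding the interaction input for over five seconds enables collision on the BP_Body actor once, unlocking it after cleaning.
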(event OnComponentBeginOverlap(Box)
  (params (OverlappedComponent :type Primitive%20Component%20Object%20Reference) (OtherActor :type Actor%20Object%20Reference) (OtherComp :type Primitive%20Component%20Object%20Reference) (OtherBodyIndex :type Integer) (bFromSweep :type Boolean) (SweepResult :type Hit%20Result%20Structure%20%28by%20ref%29))
  (Variables|/Script/UMG.Widget|SetVisibility (stale EventBeginPlay _returnvalue) "Visible"))

(event OnComponentEndOverlap(Box)
  (params (OverlappedComponent :type Primitive%20Component%20Object%20Reference) (OtherActor :type Actor%20Object%20Reference) (OtherComp :type Primitive%20Component%20Object%20Reference) (OtherBodyIndex :type Integer))
  (Variables|/Script/UMG.Widget|SetVisibility (stale EventBeginPlay _returnvalue) "Hidden"))

(event Input|EnhancedActionEvents|EnhancedInputActionIA_Interaction
  (params (ActionValue :type Boolean) (ElapsedSeconds :type Float%20%28double-precision%29) (TriggeredSeconds :type Float%20%28double-precision%29) (InputAction :type Input%20Action%20Object%20Reference :default "/Game/_Game/Input/IA_Interaction.IA_Interaction"))
  ;[0.15 0.15 0.15 0.5] This is how to do code for the cleaning and enabling the collsion of the body
  (:Triggered
    (if (Collision|IsOverlappingActor (Variables|Default|GetBox) (Game|GetPlayerCharacter 0) :!class /Script/Engine.PrimitiveComponent)
      (switch Utilities|FlowControl|Switch|SwitchonE_MaskState (Variables|/Game/_Game/Blueprints/BP_Player_NM.BP_Player_NM_C|GetCurrentMaskState (Variables|Default|GetAs%20BP%20Player%20NM))
        (:NewEnumerator1
          (Development|PrintString (Utilities|String|ToString(Float) ElapsedSeconds))
          (if (> ElapsedSeconds 5.0)
            (Development|PrintString "Task Completed Give them a number and now enable collision on the body")
            (Utilities|FlowControl|DoOnce false
              (:Completed
                (bind _returnvalue (Actor|GetActorOfClass "/Game/_Game/Blueprints/BP_Body.BP_Body_C"))
                (Default|EnableCollison _returnvalue)))))))))

(event EventBeginPlay
  (Input|EnableInput (Game|GetPlayerController 0))
  (bind _asbp_player_nm (Utilities|Casting|CastToBP_Player_NM (Game|GetPlayerCharacter 0)))
  (Variables|Default|SetAs%20BP%20Player%20NM _asbp_player_nm)
  (bind _returnvalue (UserInterface|CreateWidget "/Game/_Game/Blueprints/Interaction/WBP_UseMAsk.WBP_UseMAsk_C"))
  (UserInterface|Viewport|AddtoViewport _returnvalue 0)
  (Variables|/Script/UMG.Widget|SetVisibility _returnvalue "Hidden"))

(event EventTick
  (params (DeltaSeconds :type Float%20%28single-precision%29))
  (bind _flowerpot1 (Variables|Default|Getflowerpot1))
  (switch Utilities|FlowControl|Switch|SwitchonE_MaskState (Variables|/Game/_Game/Blueprints/BP_Player_NM.BP_Player_NM_C|GetCurrentMaskState (Variables|Default|GetAs%20BP%20Player%20NM))
    (:NewEnumerator0
      (Components|StaticMesh|SetStaticMesh _flowerpot1 "/Game/_Game/Art/Models/flowerpot1.flowerpot1")
      (Variables|/Script/UMG.TextBlock|SetText (Variables|/Game/_Game/Blueprints/Interaction/WBP_UseMAsk.WBP_UseMAsk_C|GetTextBlock_0 (stale EventBeginPlay _returnvalue)) "Maybe I should try a Mask"))
    (:NewEnumerator1
      (Components|StaticMesh|SetStaticMesh _flowerpot1 "/Game/_Game/Art/Models/Carving_knife.Carving_knife")
      (Variables|/Script/UMG.TextBlock|SetText (Variables|/Game/_Game/Blueprints/Interaction/WBP_UseMAsk.WBP_UseMAsk_C|GetTextBlock_0 (stale EventBeginPlay _returnvalue)) "Hold E to Clean"))))

(fn ConstructionScript)