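; BP_Icon is an interaction icon that changes with the player character's proximity.
; Two overlap spheres, sized from radius variables in the construction script, toggle the Outerinteract and Innerinteract visuals.
; Entering the outer sphere shows Outerinteract, and the inner sphere swaps it for Innerinteract until exit.
; The outer exit compares the player to OverlappedComponent rather than the other actor, so its hide step does not trigger.
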(event OnComponentBeginOverlap(InnerSphere)
  (params (OverlappedComponent :type Primitive%20Component%20Object%20Reference) (OtherActor :type Actor%20Object%20Reference) (OtherComp :type Primitive%20Component%20Object%20Reference) (OtherBodyIndex :type Integer) (bFromSweep :type Boolean) (SweepResult :type Hit%20Result%20Structure%20%28by%20ref%29))
  (if (== OtherActor (Game|GetPlayerCharacter 0))
    (Rendering|SetVisibility (Variables|Default|GetInnerinteract) true false)
    (Rendering|SetVisibility (Variables|Default|GetOuterinteract) false false)))

(event OnComponentEndOverlap(InnerSphere)
  (params (OverlappedComponent :type Primitive%20Component%20Object%20Reference) (OtherActor :type Actor%20Object%20Reference) (OtherComp :type Primitive%20Component%20Object%20Reference) (OtherBodyIndex :type Integer))
  (if (== (Game|GetPlayerCharacter 0) OtherActor)
    (Rendering|SetVisibility (Variables|Default|GetInnerinteract) false false)
    (Rendering|SetVisibility (Variables|Default|GetOuterinteract) true false)))

(event OnComponentBeginOverlap(OuterSphere)
  (params (OverlappedComponent :type Primitive%20Component%20Object%20Reference) (OtherActor :type Actor%20Object%20Reference) (OtherComp :type Primitive%20Component%20Object%20Reference) (OtherBodyIndex :type Integer) (bFromSweep :type Boolean) (SweepResult :type Hit%20Result%20Structure%20%28by%20ref%29))
  (if (== OtherActor (Game|GetPlayerCharacter 0))
    (Rendering|SetVisibility (Variables|Default|GetOuterinteract) true false)))

(event OnComponentEndOverlap(OuterSphere)
  (params (OverlappedComponent :type Primitive%20Component%20Object%20Reference) (OtherActor :type Actor%20Object%20Reference) (OtherComp :type Primitive%20Component%20Object%20Reference) (OtherBodyIndex :type Integer))
  (if (== (Game|GetPlayerCharacter 0) OverlappedComponent)
    (Rendering|SetVisibility (Variables|Default|GetOuterinteract) false false)))

(fn ConstructionScript
  (Components|Sphere|SetSphereRadius (Variables|Default|GetInnerSphere) (Variables|Public|GetInner%20Sphere%20Radius) true)
  (Components|Sphere|SetSphereRadius (Variables|Default|GetOuterSphere) (Variables|Public|Getouter%20Sphere%20Radius) true))