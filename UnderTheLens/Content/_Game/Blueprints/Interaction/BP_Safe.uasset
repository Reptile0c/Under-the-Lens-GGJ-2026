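; BP_Safe is an interactable safe that opens a lock code screen when usable.
; Overlapping its Box toggles an interaction prompt widget created on BeginPlay.
; Completing IA_Interaction inside the Box checks CanUse, then either shows the WBP_LockCode widget with mouse cursor and Game and UI input, or shows WBP_NoWork.
; A DoOnce reset after a short delay keeps the WBP_NoWork message from stacking.
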(event OnComponentBeginOverlap(Box)
  (params (OverlappedComponent :type Primitive%20Component%20Object%20Reference) (OtherActor :type Actor%20Object%20Reference) (OtherComp :type Primitive%20Component%20Object%20Reference) (OtherBodyIndex :type Integer) (bFromSweep :type Boolean) (SweepResult :type Hit%20Result%20Structure%20%28by%20ref%29))
  (Variables|/Script/UMG.Widget|SetVisibility (stale EventBeginPlay _returnvalue) "Visible"))

(event OnComponentEndOverlap(Box)
  (params (OverlappedComponent :type Primitive%20Component%20Object%20Reference) (OtherActor :type Actor%20Object%20Reference) (OtherComp :type Primitive%20Component%20Object%20Reference) (OtherBodyIndex :type Integer))
  (Variables|/Script/UMG.Widget|SetVisibility (stale EventBeginPlay _returnvalue) "Hidden"))

(event Input|EnhancedActionEvents|EnhancedInputActionIA_Interaction
  (params (ActionValue :type Boolean) (ElapsedSeconds :type Float%20%28double-precision%29) (TriggeredSeconds :type Float%20%28double-precision%29) (InputAction :type Input%20Action%20Object%20Reference :default "/Game/_Game/Input/IA_Interaction.IA_Interaction"))
  (bind _returnvalue (Game|GetPlayerController 0))
  (:Completed
    (if (Collision|IsOverlappingActor (Variables|Default|GetBox) (Game|GetPlayerCharacter 0) :!class /Script/Engine.PrimitiveComponent)
      (if (Variables|Default|GetCanUse?)
        (bind _returnvalue_2 (UserInterface|CreateWidget "/Game/_Game/UI/WBP_LockCode.WBP_LockCode_C"))
        (UserInterface|Viewport|AddtoViewport _returnvalue_2 0)
        (Variables|/Script/Engine.PlayerController|SetbShowMouseCursor _returnvalue true)
        (Input|SetInputModeGameandUI _returnvalue _returnvalue_2 "DoNotLock" true false)
        (else
          (Utilities|FlowControl|DoOnce false :!label _label
            (:Completed
              (bind _returnvalue_3 (UserInterface|CreateWidget "/Game/_Game/Blueprints/Interaction/WBP_NoWork.WBP_NoWork_C"))
              (UserInterface|Viewport|AddtoViewport _returnvalue_3 0)
              (Utilities|FlowControl|Delay 2.1)
              (goto _label Reset))))))))

(event EventBeginPlay
  (Input|EnableInput (Game|GetPlayerController 0))
  (bind _returnvalue (UserInterface|CreateWidget "/Game/_Game/Blueprints/Interaction/WBP_Interect.WBP_Interect_C"))
  (UserInterface|Viewport|AddtoViewport _returnvalue 0)
  (Variables|/Script/UMG.Widget|SetVisibility _returnvalue "Hidden"))

(fn ConstructionScript)