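; BP_Item is a configurable interactable world item that can be inspected, with pickup only stubbed as a debug print.
; The construction script applies the item's mesh and scale.
; When Inspect is set, Interaction spawns a BP_Inspectitem at a far-off location and passes it the character, mesh, name, description, inspection rotation and scale.
; BeginPlay's player cast has no target class and stores no character reference.
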(event EventBeginPlay
  (bind _asbp_first_person_character (Utilities|Casting|CastTo (Game|GetPlayerCharacter 0)))
  (Variables|Public|Reference|SetAs%20BP%20First%20Person%20Character 0 _asbp_first_person_character))

(event EventInteraction
  (params (Character :type Object%20Object%20Reference))
  (if (Variables|Public|Interaction|Inspection|Getinspect?)
    (bind _returnvalue (Game|SpawnActorfromClass "/Game/_Game/Input/Inspect/BP_Inspectitem.BP_Inspectitem_C" (Math|Transform|MakeTransform "1000000000.000000,0.000000,0.000000") "Undefined" "MultiplyWithRoot" 0 0))
    (Default|SetInspectRotation _returnvalue (Variables|Public|Interaction|Inspection|GetItemInspectionRotation))
    (Default|SetInspectScale _returnvalue (Variables|Public|Interaction|Inspection|GetInspectionScale))
    (Class|InteractionInterface|Inspect(Message) _returnvalue Character (Variables|/Script/Engine.StaticMeshComponent|GetStaticMesh (Variables|Default|GetStaticMesh)) (Variables|Public|Mesh|GetItemName) (Variables|Public|Mesh|GetItemDescription))
    (else
      (Development|PrintString "PickUp"))))

(fn ConstructionScript
  (bind _staticmesh (Variables|Default|GetStaticMesh))
  ;[1 1 1] SettingMesh
  (Components|StaticMesh|SetStaticMesh (Variables|Default|GetStaticMesh) (Variables|Public|Mesh|GetitemMesh))
  ;[1 1 1] setting scale
  (Transformation|SetWorldTransform _staticmesh (Math|Transform|MakeTransform (Transformation|GetWorldLocation _staticmesh) (Transformation|GetWorldRotation _staticmesh) (Variables|Public|Mesh|GetItemScale)) false false))