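; BP_Masks is an interactable mask actor that the player uses by pressing E while standing inside its Box volume.
; It enables input from the first player controller at BeginPlay, then checks player character overlap on each key press.
; A successful press passes its MaskState to the player controller's EnableTheMasksUIMessage, then destroys the actor after a short delay.
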(event EventBeginPlay
  (Input|EnableInput (Game|GetPlayerController 0)))

(event Input|KeyboardEvents|E
  (params (Key :type Key%20Structure :default "None"))
  (:Pressed
    (if (Collision|IsOverlappingActor (Variables|Default|GetBox) (Game|GetPlayerCharacter 0) :!class /Script/Engine.PrimitiveComponent)
      (Class|BIPlayerInterfaces|EnabletheMasksUI(Message) (Game|GetPlayerController 0) (Variables|Default|GetMaskState))
      (Utilities|FlowControl|Delay 0.2)
      (Actor|DestroyActor))))

(fn ConstructionScript)