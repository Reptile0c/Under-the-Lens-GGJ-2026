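; Note1 is an interactable note that the player opens and closes to read on screen.
; Its Interaction event runs a FlipFlop that alternates between the two states.
; Opening plays a pickup sound at the Cube, adds a Notewidget to the viewport, and blocks look and move input.
; Closing plays a drop sound, removes the widget, and restores input.
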(event EventInteraction
  (params (Character :type Object%20Object%20Reference))
  (bind _returnvalue (Game|GetPlayerController 0))
  (bind _cube (Variables|Default|GetCube))
  (bind _returnvalue_2 (Transformation|GetWorldLocation _cube))
  (Utilities|FlowControl|FlipFlop
    (:A
      (Audio|PlaySoundatLocation "/Game/_Game/Audio/pickupnote.pickupnote" _returnvalue_2 "0, 0, 0" 1.0 1.0 0.0 0 0 0 0)
      (bind _returnvalue_3 (UserInterface|CreateWidget "/Game/_Game/Blueprints/Interaction/Notewidget.Notewidget_C"))
      (UserInterface|Viewport|AddtoViewport _returnvalue_3 0)
      (Input|SetIgnoreLookInput _returnvalue true)
      (Input|SetIgnoreMoveInput _returnvalue true))
    (:B
      (Audio|PlaySoundatLocation "/Game/_Game/Audio/dropnote.dropnote" _returnvalue_2 "0, 0, 0" 1.0 1.0 0.0 0 0 0 0)
      (Widget|RemovefromParent _returnvalue_3)
      (Input|SetIgnoreLookInput _returnvalue false)
      (Input|SetIgnoreMoveInput _returnvalue false))))

(fn ConstructionScript)