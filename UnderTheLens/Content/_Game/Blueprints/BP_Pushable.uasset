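; BP_Pushable is a pushable locker that slides a set distance when the player walks into it head-on.
; On hit, it rounds the player's forward vector into a push direction, then CanPush line-traces for the locker and box-traces for a clear path.
; A valid push disables player movement and attaches the player while a Timeline moves the locker with sound.
; When the Timeline finishes, the sound stops and the player detaches and walks again.
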(event Custom|Push
  (bind _returnvalue (Transformation|GetActorLocation))
  (Utilities|FlowControl|Sequence
    (:then_0
      (Variables|Default|SetCurrentLocation _returnvalue)
      (bind _newtrack_0 (Timeline|Timeline Play)
        (:Update
          (Transformation|SetActorRelativeLocation (+ (Variables|Default|GetCurrentLocation) (* _newtrack_0 (Variables|Default|GetpushableDirection) (Variables|Default|GettravelDistance)))))
        (:Finished
          (CallFunction|Stoppushing))))
    (:then_1
      (Utilities|IsValid (Variables|Default|GetNewVar)
        (:Is%20Not%20Valid
          (bind _returnvalue_2 (Audio|SpawnSoundatLocation "/Engine/VREditor/Sounds/VR_objectRotateLoop_01.VR_objectRotateLoop_01" _returnvalue "0, 0, 0" 1.0 1.0 0.0 0 0))
          (Variables|Default|SetNewVar _returnvalue_2))))))

(event Custom|stoppushing
  (bind _returnvalue (Game|GetPlayerCharacter 0))
  (Audio|Components|Audio|Stop (Variables|Default|GetNewVar))
  (Pawn|Components|CharacterMovement|SetMovementMode (Variables|/Script/Engine.Character|GetCharacterMovement _returnvalue) "MOVE_Walking" 0)
  (Transformation|DetachFromActor _returnvalue "KeepWorld" "KeepWorld" "KeepWorld"))

(event Collision|EventHit
  (params (MyComp :type Primitive%20Component%20Object%20Reference) (Other :type Actor%20Object%20Reference) (OtherComp :type Primitive%20Component%20Object%20Reference) (bSelfMoved :type Boolean) (HitLocation :type Vector :default "0, 0, 0") (HitNormal :type Vector :default "0, 0, 0") (NormalImpulse :type Vector :default "0, 0, 0") (Hit :type Hit%20Result%20Structure%20%28by%20ref%29))
  (bind _returnvalue (Transformation|GetActorForwardVector Other))
  (bind _returnvalue_2 (Game|GetPlayerCharacter 0))
  (bind (_x _y _z) (Math|Vector|BreakVector _returnvalue))
  (if (== (Game|GetPlayerCharacter 0) Other)
    (if (> (Math|Vector|DotProduct HitNormal _returnvalue) 0.93)
      (Variables|Default|SetpushableDirection (Math|Vector|MakeVector (Math|Conversions|ToFloat(Integer) (Math|Float|Round _x)) (Math|Conversions|ToFloat(Integer) (Math|Float|Round _y)) (Math|Conversions|ToFloat(Integer) (Math|Float|Round _z))))
      (bind _canpush (CallFunction|CanPush))
      (if _canpush
        (Pawn|Components|CharacterMovement|DisableMovement (Variables|/Script/Engine.Character|GetCharacterMovement _returnvalue_2))
        (Transformation|AttachActorToActor _returnvalue_2 self "None" "KeepWorld" "KeepWorld" "KeepWorld" true)
        (CallFunction|Push)))))

(fn ConstructionScript)

(fn CanPush
  (bind _returnvalue (Game|GetPlayerCharacter 0))
  (bind _returnvalue_2 (Transformation|GetActorLocation))
  (bind _moveablelocker (Variables|Default|GetMoveableLocker))
  (bind _returnvalue_3 (Transformation|GetActorLocation _returnvalue))
  (bind (_outhit _returnvalue_4) (Collision|LineTraceByChannel _returnvalue_3 (+ _returnvalue_3 (* (Transformation|GetActorForwardVector _returnvalue) 8e+01)) "TraceTypeQuery1" false (Utilities|Array|MakeArray _returnvalue) "ForDuration" false))
  (if _returnvalue_4
    (if (== (.HitActor (Collision|BreakHitResult _outhit)) self)
      (bind _returnvalue_5 (Collision|BoxTraceByChannel (+ _returnvalue_2 (Math|Vector|MakeVector -1e+02 -1e+02 2e+02)) (+ _returnvalue_2 (* (Variables|Default|GetpushableDirection) (Variables|Default|GettravelDistance)) (Math|Vector|MakeVector -1e+02 -1e+02 2e+02)) (* (.boxextent (StaticMesh|GetBounds (Variables|/Script/Engine.StaticMeshComponent|GetStaticMesh _moveablelocker))) (Variables|/Script/Engine.SceneComponent|GetRelativeScale3D _moveablelocker) "0.900000,0.900000,0.900000") "0, 0, 0" "TraceTypeQuery1" false 0 "ForDuration"))
      (return (not _returnvalue_5))
      (else
        (return false)))
    (else
      (return false))))