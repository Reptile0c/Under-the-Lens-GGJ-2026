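; Item inspection actor that displays a given mesh with its name and description in a W_Inspect widget.
; Holding left mouse rotates the item, the wheel zooms by changing the SceneCapture camera's clamped FOV, and right mouse resets rotation and zoom.
; Separate events set the item's starting rotation and scale.
; The Interaction event restores character input, removes the widget and destroys the actor.
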(event Custom|Set%20inspect%20rotation
  (params (ItemRotation :type Rotator))
  (bind _item (Variables|Default|GetItem))
  (bind _returnvalue (Transformation|GetWorldTransform _item))
  ;[1 1 1] set inspection rotation
  (bind _output_get (Variables|Default|Setinitial%20Rotation ItemRotation))
  (Transformation|SetWorldTransform _item (Math|Transform|MakeTransform (.location _returnvalue) _output_get (.scale _returnvalue)) false false))

(event Custom|Set%20inspect%20scale
  (params (inspection%20scale :type Vector))
  (bind _item (Variables|Default|GetItem))
  (bind _returnvalue (Transformation|GetWorldTransform _item))
  (Transformation|SetWorldTransform _item (Math|Transform|MakeTransform (.location _returnvalue) (.rotation _returnvalue) inspection%20scale) false false))

(event EventInspect
  (params (Character :type Object%20Object%20Reference) (InspectedItem :type Static%20Mesh%20Object%20Reference) (Item%20name :type Text) (Item%20description :type Text))
  (bind _returnvalue (Game|GetPlayerController 0))
  (Variables|Default|SetCharacter 0 Character)
  (Components|StaticMesh|SetStaticMesh (Variables|Default|GetItem) InspectedItem)
  (bind _returnvalue_2 (UserInterface|CreateWidget "/Game/_Game/Input/Inspect/W_Inspect.W_Inspect_C" 0 Item%20name Item%20description))
  (bind _output_get (Variables|Default|SetInspectwidgetreference _returnvalue_2))
  (UserInterface|Viewport|AddtoViewport _output_get 0)
  (Input|DisableInput _returnvalue)
  (Input|EnableInput (.Character (Variables|Default|GetCharacter)) _returnvalue))

(event EventInteraction
  (params (Character :type Object%20Object%20Reference))
  (bind _returnvalue (Game|GetPlayerController 0))
  (Input|DisableInput _returnvalue)
  (Input|EnableInput (.Character (Variables|Default|GetCharacter)) _returnvalue)
  (Utilities|IsValid (Variables|Default|GetInspectwidgetreference)
    (:Is%20Valid
      (Widget|RemovefromParent (Variables|Default|GetInspectwidgetreference))
      (Variables|Default|SetInspectwidgetreference 0)
      (Actor|DestroyActor))))

(event Input|MouseEvents|MouseX
  (params (AxisValue :type Float%20%28single-precision%29))
  ;[1 1 1] Set mouse movement horizontally
  (if (Variables|Default|GetRotate?)
    (Transformation|SetWorldRotation (Variables|Default|GetItem) (Math|Rotator|CombineRotators (Transformation|GetWorldRotation (Variables|Default|GetItem)) (Math|Rotator|MakeRotator 0.0 0.0 (* AxisValue -3.0))) false false)))

(event Input|MouseEvents|MouseY
  (params (AxisValue :type Float%20%28single-precision%29))
  ;[1 1 1] Set mouse movement vertically
  (if (Variables|Default|GetRotate?)
    (Transformation|SetWorldRotation (Variables|Default|GetItem) (Math|Rotator|CombineRotators (Transformation|GetWorldRotation (Variables|Default|GetItem)) (Math|Rotator|MakeRotator 0.0 (* AxisValue -3.0) 0.0)) false false)))

(event Input|MouseEvents|LeftMouseButton
  (params (Key :type Key%20Structure))
  ;[1 1 1] Only allow
  (:Pressed
    (Variables|Default|SetRotate? true))
  (:Released
    (Variables|Default|SetRotate? false)))

(event Input|MouseEvents|RightMouseButton
  (params (Key :type Key%20Structure))
  ;[1 1 1] Reseting transform of the item
  (:Pressed
    (Transformation|SetWorldRotation (Variables|Default|GetItem) (Variables|Default|Getinitial%20Rotation) false false)
    (Variables|/Script/Engine.SceneCaptureComponent2D|SetFOVAngle (Variables|Default|GetSceneCaptureComponent2D) 5e+01)))

(event Input|MouseEvents|MouseWheelUp
  (params (Key :type Key%20Structure))
  (bind _scenecapturecomponent2d (Variables|Default|GetSceneCaptureComponent2D))
  ;[1 1 1] Zoom in
  (:Pressed
    (Variables|/Script/Engine.SceneCaptureComponent2D|SetFOVAngle _scenecapturecomponent2d (Math|Float|Clamp(Float) (- (Variables|/Script/Engine.SceneCaptureComponent2D|GetFOVAngle _scenecapturecomponent2d) 1.0) 3e+01 8e+01))))

(event Input|MouseEvents|MouseWheelDown
  (params (Key :type Key%20Structure))
  (bind _scenecapturecomponent2d (Variables|Default|GetSceneCaptureComponent2D))
  ;[1 1 1] zoom out
  (:Pressed
    (Variables|/Script/Engine.SceneCaptureComponent2D|SetFOVAngle _scenecapturecomponent2d (Math|Float|Clamp(Float) (+ (Variables|/Script/Engine.SceneCaptureComponent2D|GetFOVAngle _scenecapturecomponent2d) 1.0) 3e+01 8e+01))))

(fn ConstructionScript)